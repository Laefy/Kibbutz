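; RunningGuyTrigger_BP is a one-shot trigger volume that plays the RunningGuy_LS level sequence.
; When the first player character's capsule overlaps its collision component, a Done flag prevents repeats and a sequence player is created.
; It blocks input through MainController while the sequence plays and restores it from the player's OnStop event.
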(event `self.CollisionComponent.OnComponentBeginOverlap`
  (params (OverlappedComponent :type "PrimitiveComponent Object Reference") (OtherActor :type "Actor Object Reference") (OtherComp :type "PrimitiveComponent Object Reference") (OtherBodyIndex :type Integer) (bFromSweep :type Boolean) (SweepResult :type "HitResult Structure (by ref)"))
  (bind _returnvalue (`GameplayStatics.GetPlayerCharacter` 0))
  (if (and (not (`self.Done`)) (== OtherActor _returnvalue) (== OtherComp (`Character.CapsuleComponent` _returnvalue)))
    (set `self.Done` true)
    (bind _returnvalue_2 (`LevelSequencePlayer.CreateLevelSequencePlayer` "/Game/Cinematics/Night1/RunningGuy_LS.RunningGuy_LS"))
    (bind _asmain_controller (cast `MainController` (`GameplayStatics.GetPlayerController` 0)))
    (`MainController.BlockInputs` _asmain_controller true)
    (add `LevelSequencePlayer.OnStop` _returnvalue_2 (delegate `Event_End`))
    (`LevelSequencePlayer.Play` _returnvalue_2)))

(event `Event_End`
  (`MainController.BlockInputs` (stale `self.CollisionComponent.OnComponentBeginOverlap` _asmain_controller) false))

(fn `UserConstructionScript`)