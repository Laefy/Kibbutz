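; Door trigger actor that asks the player whether to go back to bed when their character steps into it.
; On BeginPlay it creates a CinematicUI choice widget, sets the question with two answers and binds both buttons.
; Overlap begin and end add or remove the widget while Active is true.
; Confirming hides it and calls GoToBed; declining only hides it.
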(event `Event_GoToBed`
  (`Widget.RemoveFromParent` (`self.UI`))
  (`self.GoToBed`))

(event `ContinueWandering`
  (`Widget.RemoveFromParent` (`self.UI`)))

(event `self.ReceiveBeginPlay`
  (bind _returnvalue (`|CreateWidget` "/Game/Menu/Cinematic/CinematicUI.CinematicUI_C" (`GameplayStatics.GetPlayerController` 0)))
  (bind _output_get (set `self.UI` _returnvalue))
  (add `Button.OnClicked` (`/Game/Menu/Cinematic/CinematicUI.Action1` _output_get) (delegate `Event_GoToBed`))
  (add `Button.OnClicked` (`/Game/Menu/Cinematic/CinematicUI.Action2` _output_get) (delegate `ContinueWandering`))
  (`/Game/Menu/Cinematic/CinematicUI.SetChoice` _output_get "Go back to bed ?" "Yes, I'm tired now." "No ! I have plenty of things left to do !"))

(event `self.ReceiveActorBeginOverlap`
  (params (OtherActor :type "Actor Object Reference"))
  (if (and (== (`GameplayStatics.GetPlayerCharacter` 0) OtherActor) (`self.Active`))
    (`UserWidget.AddToViewport` (`self.UI`) 0)))

(event `self.ReceiveActorEndOverlap`
  (params (OtherActor :type "Actor Object Reference"))
  (if (and (== (`GameplayStatics.GetPlayerCharacter` 0) OtherActor) (`self.Active`))
    (`Widget.RemoveFromParent` (`self.UI`))))

(fn `UserConstructionScript`)