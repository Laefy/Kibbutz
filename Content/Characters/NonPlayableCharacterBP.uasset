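; Non-playable character that holds branching, day-specific dialogue with the player and can hand out quests.
; Entering its box shows the current NPCStatements line and up to three response buttons, if the game mode's clock matches that statement's day.
; Responses jump via GoToStatement indices, while the OnBecomeDay event selects the new day's first statement.
; Statement quests are found by object-name substring among Quest actors and added to MainController.
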(event `RespondEvent3`
  ;[1 1 1] On response click
  (`self.Respond` 2))

(event `OnBecomeDay`
  (params (Day :type Byte))
  ;[1 1 1] Handle synchronization between day and dialogue. e.g : when day set currentstatement to day two first dialogue
  (for (_array_element _array_index) (`self.NPCStatements`) :!label _label
    (if (== Day (`KismetMathLibrary.Conv_IntToByte` (`.Day` (break `NPCStatement` _array_element))))
      (set `self.CurrentStatement` _array_index)
      (break))))

(event `RespondEvent2`
  ;[1 1 1] On response click
  (`self.Respond` 1))

(event `RespondEvent1`
  ;[1 1 1] On response click
  (`self.Respond` 0))

(event `self.ReceiveBeginPlay`
  (bind _verticaloptionsbox (`/Game/NPCDialogue/Blueprints/PlayerOptions.VerticalOptionsBox` (`self.OptionsWidget`)))
  (`self.CreateWidgets`)
  ;[1 1 1] On response click
  (bind _asbutton (cast `Button` (`PanelWidget.GetChildAt` _verticaloptionsbox 0)))
  (add `Button.OnClicked` _asbutton (delegate `RespondEvent1`))
  (bind _asbutton_2 (cast `Button` (`PanelWidget.GetChildAt` _verticaloptionsbox 1)))
  (add `Button.OnClicked` _asbutton_2 (delegate `RespondEvent2`))
  (bind _asbutton_3 (cast `Button` (`PanelWidget.GetChildAt` _verticaloptionsbox 2)))
  (add `Button.OnClicked` _asbutton_3 (delegate `RespondEvent3`))
  ;[1 1 1] Handle synchronization between day and dialogue. e.g : when day set currentstatement to day two first dialogue
  (bind _askibbutz_game_mode (cast `KibbutzGameMode` (`GameplayStatics.GetGameMode`)))
  (add `KibbutzGameMode.OnBecomeDay` _askibbutz_game_mode (delegate `OnBecomeDay`))
  (goto _label))

(event `self.Box.OnComponentBeginOverlap`
  (params (OverlappedComponent :type "PrimitiveComponent Object Reference") (OtherActor :type "Actor Object Reference") (OtherComp :type "PrimitiveComponent Object Reference") (OtherBodyIndex :type Integer) (bFromSweep :type Boolean) (SweepResult :type "HitResult Structure (by ref)"))
  (if (== OtherActor (`GameplayStatics.GetPlayerCharacter` 0))
    (`self.ShowOptions`)))

(event `self.Box.OnComponentEndOverlap`
  (params (OverlappedComponent :type "PrimitiveComponent Object Reference") (OtherActor :type "Actor Object Reference") (OtherComp :type "PrimitiveComponent Object Reference") (OtherBodyIndex :type Integer))
  (if (== OtherActor (`GameplayStatics.GetPlayerCharacter` 0))
    (`Widget.SetVisibility` (`self.OptionsWidget`) "Hidden")
    (`Widget.SetVisibility` (`self.DialogueWidget`) "Hidden")
    (set `self.WaitingForResponse` false)))

(fn `ActivateQuest`
  (params (QuestName :type String))
  (bind _outactors (`GameplayStatics.GetAllActorsOfClass` "/Script/Kibbutz.Quest"))
  (for _array_element _outactors
    (if (>= (`KismetStringLibrary.FindSubstring` (`KismetSystemLibrary.GetObjectName` _array_element) QuestName) 0)
      (bind _asmain_controller (cast `MainController` (`GameplayStatics.GetPlayerController` 0))
        (:`then`
          (`MainController.AddQuest` _asmain_controller _array_element :!pinned true) ; Activate quest
          (break))
        (:`CastFailed`
          (`KismetSystemLibrary.PrintString` "Cast failed: Activate quest --> PlayerController to MainController" false))))))

(fn `ClearOptions`
  (bind _verticaloptionsbox (`/Game/NPCDialogue/Blueprints/PlayerOptions.VerticalOptionsBox` (`self.OptionsWidget`)))
  (bind _asbutton (cast `Button` (`PanelWidget.GetChildAt` _verticaloptionsbox 2)))
  (bind _astext (cast `TextBlock` (`PanelWidget.GetChildAt` _asbutton 0)))
  (`TextBlock.SetText` _astext "")
  (`Widget.SetVisibility` _asbutton "Hidden")
  (bind _asbutton_2 (cast `Button` (`PanelWidget.GetChildAt` _verticaloptionsbox 1)))
  (bind _astext_2 (cast `TextBlock` (`PanelWidget.GetChildAt` _asbutton_2 0)))
  (`TextBlock.SetText` _astext_2 "")
  (`Widget.SetVisibility` _asbutton_2 "Hidden")
  (bind _asbutton_3 (cast `Button` (`PanelWidget.GetChildAt` _verticaloptionsbox 0)))
  (bind _astext_3 (cast `TextBlock` (`PanelWidget.GetChildAt` _asbutton_3 0)))
  (`TextBlock.SetText` _astext_3 "")
  (`Widget.SetVisibility` _asbutton_3 "Hidden"))

(fn `CreateWidgets`
  (`|ExecutionSequence`
    (:`then_0`
      (bind _returnvalue (`|CreateWidget` "/Game/NPCDialogue/Blueprints/DialogueText.DialogueText_C"))
      (bind _output_get (set `self.DialogueWidget` _returnvalue))
      (`UserWidget.AddToViewport` _output_get 0)
      (`Widget.SetVisibility` _output_get "Hidden")
      (`TextBlock.SetColorAndOpacity` (`/Game/NPCDialogue/Blueprints/DialogueText.Dialogue` _output_get) (`self.Color`)))
    (:`then_1`
      (bind _returnvalue_2 (`|CreateWidget` "/Game/NPCDialogue/Blueprints/PlayerOptions.PlayerOptions_C"))
      (bind _output_get_2 (set `self.OptionsWidget` _returnvalue_2))
      (`UserWidget.AddToViewport` _output_get_2 0)
      (`Widget.SetVisibility` _output_get_2 "Hidden")
      (`Widget.SetVisibility` (`PanelWidget.GetChildAt` (`/Game/NPCDialogue/Blueprints/PlayerOptions.VerticalOptionsBox` _returnvalue_2) 2) "Hidden")
      (`Widget.SetVisibility` (`PanelWidget.GetChildAt` (`/Game/NPCDialogue/Blueprints/PlayerOptions.VerticalOptionsBox` _returnvalue_2) 0) "Hidden")
      (`Widget.SetVisibility` (`PanelWidget.GetChildAt` (`/Game/NPCDialogue/Blueprints/PlayerOptions.VerticalOptionsBox` _returnvalue_2) 1) "Hidden"))))

(fn `Respond`
  (params (ResponseIndex :type Integer))
  (bind (_player_response _go_to_statement) (break `PlayerResponse` (`KismetArrayLibrary.Array_Get` (`.Player_Responses` (break `NPCStatement` (`KismetArrayLibrary.Array_Get` (`self.NPCStatements`) (`self.CurrentStatement`)))) ResponseIndex)))
  (if (>= _go_to_statement 0)
    (bind _output_get (set `self.CurrentStatement` (- _go_to_statement 1)))
    (bind (_npc_dialogue _player_responses _day _quest) (break `NPCStatement` (`KismetArrayLibrary.Array_Get` (`self.NPCStatements`) _output_get)))
    (if (> (`KismetArrayLibrary.Array_Length` _player_responses) 0)
      ;[1 1 1] Still something to say
      (`self.ShowOptions`)
      (else
        (`self.Talk` _npc_dialogue _quest)
        ;[1 1 1] End
        (set `self.WaitingForResponse` false :!label _label)
        (set `self.CurrentStatement` (- (`KismetMathLibrary.Abs_Int` _go_to_statement) 1))
        (`Widget.SetVisibility` (`self.OptionsWidget`) "Hidden")))
    (else
      (goto _label))))

(fn `ShowOptions`
  (bind _npcstatements (`self.NPCStatements`))
  (bind _currentstatement (`self.CurrentStatement`))
  (bind (_npc_dialogue _player_responses _day _quest) (break `NPCStatement` (`KismetArrayLibrary.Array_Get` _npcstatements _currentstatement)))
  ;[1 1 1] Check that the dialog is allowed given which day the game is
  (bind _askibbutz_game_mode (cast `KibbutzGameMode` (`GameplayStatics.GetGameMode`)))
  (bind _clock_days (break `ClockStruct` (`KibbutzGameMode.Clock` _askibbutz_game_mode)))
  (if (== _clock_days _day)
    (if (< _currentstatement (`KismetArrayLibrary.Array_Length` _npcstatements))
      (`self.Talk` _npc_dialogue _quest)
      (`self.ClearOptions`)
      (for (_array_element _array_index) _player_responses
        (bind _asbutton (cast `Button` (`PanelWidget.GetChildAt` (`/Game/NPCDialogue/Blueprints/PlayerOptions.VerticalOptionsBox` (`self.OptionsWidget`)) _array_index)))
        (bind _astext (cast `TextBlock` (`PanelWidget.GetChildAt` _asbutton 0)))
        (`TextBlock.SetText` _astext (`.Player_Response` (break `PlayerResponse` _array_element)))
        (`Widget.SetVisibility` _asbutton "Visible"))
      (`Widget.SetVisibility` (`self.OptionsWidget`) "Visible")
      (set `self.WaitingForResponse` false))))

(fn `Talk`
  (params (Text :type Text) (Quest :type String))
  (bind _dialoguewidget (`self.DialogueWidget`))
  (`TextBlock.SetText` (`/Game/NPCDialogue/Blueprints/DialogueText.Dialogue` _dialoguewidget) (`KismetTextLibrary.Conv_StringToText` (`KismetStringLibrary.Concat_StrStr` (`KismetStringLibrary.Concat_StrStr` (`self.FriendlyName`) ": ") (`KismetTextLibrary.Conv_TextToString` Text))))
  (`Widget.SetVisibility` _dialoguewidget "Visible")
  (if (`KismetStringLibrary.NotEqual_StrStr` Quest)
    (`self.ActivateQuest` Quest)))

(fn `UserConstructionScript`)