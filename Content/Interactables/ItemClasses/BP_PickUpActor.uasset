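; World pickup actor that adds an amount of an item class to the character's inventory, with a widget showing item name and amount.
; Sphere overlaps maintain MainCharacterBP's NearbyPickupActors queue, so only the first entry shows its prompt.
; OnPickedUp keeps any leftover amount and refreshes the text, or leaves the queue, reveals the next prompt and destroys itself.
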(event `self.ReceiveBeginPlay`
  (`self.UpdateText`))

(event `OnPickedUp`
  (params (Character :type "/Game/Characters/MainCharacterBP Object Reference"))
  (bind _inventoryref (`/Game/Characters/MainCharacterBP.InventoryRef` Character))
  (bind _nearbypickupactors (`/Game/Characters/MainCharacterBP.NearbyPickupActors` Character))
  (bind _item (`KismetArrayLibrary.Array_Get` _nearbypickupactors))
  (`/Engine/EditorBlueprintResources/StandardMacros.IsValid` _inventoryref
    (:`Is Valid`
      (bind (_success_ _rest) (`/Game/Interactables/BP_Inventory.AddItem` _inventoryref (`self.ItemToAdd`) (`self.Amount`)))
      (if _success_
        (if (> _rest 0)
          (set `self.Amount` _rest)
          (`self.UpdateText`)
          (else
            (`KismetArrayLibrary.Array_RemoveItem` _nearbypickupactors self)
            (`/Engine/EditorBlueprintResources/StandardMacros.IsValid` _item
              (:`Is Valid`
                (`SceneComponent.SetVisibility` (`/Game/Interactables/ItemClasses/BP_PickUpActor.PickupText` _item) true false)
                (`self.K2_DestroyActor`))
              (:`Is Not Valid`
                (`self.K2_DestroyActor`)))))))))

(event `self.Sphere.OnComponentBeginOverlap`
  (params (OverlappedComponent :type "PrimitiveComponent Object Reference") (OtherActor :type "Actor Object Reference") (OtherComp :type "PrimitiveComponent Object Reference") (OtherBodyIndex :type Integer) (bFromSweep :type Boolean) (SweepResult :type "HitResult Structure (by ref)"))
  (bind _asmain_character_bp (cast `/Game/Characters/MainCharacterBP` OtherActor))
  (bind _nearbypickupactors (`/Game/Characters/MainCharacterBP.NearbyPickupActors` _asmain_character_bp))
  (if (> (`KismetArrayLibrary.Array_Length` _nearbypickupactors) 0)
    (`KismetArrayLibrary.Array_Add` _nearbypickupactors self)
    (else
      (`SceneComponent.SetVisibility` (`self.PickupText`) true false)
      (`KismetArrayLibrary.Array_Add` _nearbypickupactors self))))

(event `self.Sphere.OnComponentEndOverlap`
  (params (OverlappedComponent :type "PrimitiveComponent Object Reference") (OtherActor :type "Actor Object Reference") (OtherComp :type "PrimitiveComponent Object Reference") (OtherBodyIndex :type Integer))
  (bind _asmain_character_bp (cast `/Game/Characters/MainCharacterBP` OtherActor))
  (bind _nearbypickupactors (`/Game/Characters/MainCharacterBP.NearbyPickupActors` _asmain_character_bp))
  (bind _item (`KismetArrayLibrary.Array_Get` _nearbypickupactors))
  (if (and (`KismetSystemLibrary.IsValid` _item) (== _item self))
    (`SceneComponent.SetVisibility` (`self.PickupText`) false false)
    (`KismetArrayLibrary.Array_RemoveItem` _nearbypickupactors self)
    (bind _item_2 (`KismetArrayLibrary.Array_Get` (`/Game/Characters/MainCharacterBP.NearbyPickupActors` _asmain_character_bp)))
    (`/Engine/EditorBlueprintResources/StandardMacros.IsValid` _item_2
      (:`Is Valid`
        (`SceneComponent.SetVisibility` (`/Game/Interactables/ItemClasses/BP_PickUpActor.PickupText` _item_2) true false)))
    (else
      (`KismetArrayLibrary.Array_RemoveItem` _nearbypickupactors self))))

(fn `UpdateText`
  (bind _asui_pickup_text (cast `/Game/UI/Inventory/UI_PickupText` (`WidgetComponent.GetUserWidgetObject` (`self.PickupText`)))
    (:`then`
      (`TextBlock.SetText` (`/Game/UI/Inventory/UI_PickupText.NameText` _asui_pickup_text) (`|FormatText` "{Item Name} ({Amount})" (`.ItemName_20_328B551B4C02CE2AD61996892E079E0E` (break `/Game/Interactables/FItemInfo` (defaults `/Game/Interactables/ItemClasses/BP_PickUpActor` (`self.ItemToAdd`)))) (`KismetTextLibrary.Conv_IntToText` (`self.Amount`)))))
    (:`CastFailed`
      _))
  (return))

(fn `UserConstructionScript`)