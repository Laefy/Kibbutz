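; Player inventory that stores items as class-and-amount slots and owns the main UI widget, which it shows and hides.
; AddItem fills free stacks, then empty slots, recursing on overflow and returning any remainder.
; RemoveItem draws an amount across matching slots, with slot changes refreshing slot widgets and often the crafting detail view.
; Item info comes from class defaults, so an item actor spawns only when used.
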(event `self.ReceiveBeginPlay`
  (bind _mainwidget (`self.MainWidget`))
  (`KismetArrayLibrary.Array_Resize` (`self.Slots`) (`self.AmountSlots`))
  (bind _returnvalue (`|CreateWidget` "/Game/UI/Inventory/UI_MainWidget.UI_MainWidget_C" null self (`self.SlotsPerRow`)))
  (bind _output_get (set `self.MainWidget` _returnvalue))
  (set `self.InventoryWidget` (`/Game/UI/Inventory/UI_MainWidget.InventoryWidget` _output_get))
  (`/Game/Characters/MainCharacterBP.UpdateGold` (`self.CharacterRef`))
  (`UserWidget.AddToViewport` _mainwidget 0)
  (`Widget.SetVisibility` _mainwidget "Hidden"))

(event `UpdateSlotAtIndex`
  (params (Index :type Integer))
  (`/Game/UI/Inventory/UI_InventorySlot.UpdateSlot` (`KismetArrayLibrary.Array_Get` (`/Game/UI/Inventory/UI_Inventory.SlotsWidgets` (`self.InventoryWidget`)) Index)))

(event `UseItemAtIndex`
  (params (Index :type Integer))
  (bind _itemclass (break `/Game/Interactables/FInventorySlot` (`KismetArrayLibrary.Array_Get` (`self.Slots`) Index)))
  (if (`KismetSystemLibrary.IsValidClass` _itemclass)
    (bind _returnvalue (`|SpawnActorFromClass` _itemclass (`KismetMathLibrary.MakeTransform` (0.0 0.0 0.0)) "AlwaysSpawn" "OverrideRootScale" null self Index))
    (`/Game/Interactables/ItemClasses/BP_BaseItem.EventOnUsed` _returnvalue)))

(fn `AddItem`
  (params (ItemClass :type "/Game/Interactables/ItemClasses/BP_BaseItem Class Reference") (Amount :type Integer))
  (returns (`Success?` :type Boolean) (Rest :type Integer))
  (locals (LocalClass :type "/Game/Interactables/ItemClasses/BP_BaseItem Class Reference") (LocalAmount :type Integer) (FoundIndex :type Integer))
  (bind _returnvalue (+ (`.Amount_3_977591134B76789C8B001BB927F69178` (break `/Game/Interactables/FInventorySlot` (`KismetArrayLibrary.Array_Get` (`self.Slots`) (`local.FoundIndex`)))) (`local.LocalAmount`)))
  (set `local.LocalClass` ItemClass)
  (set `local.LocalAmount` Amount)
  (if (`.CanBeStacked?_21_5AB843E34E1254774F491FA7A1E5A2DA` (break `/Game/Interactables/FItemInfo` (defaults `/Game/Interactables/BP_Inventory` ItemClass)))
    (bind (_success_ _index) (`self.SearchFreeStack` (`local.LocalClass`)))
    (if _success_
      (set `local.FoundIndex` _index)
      (if (> _returnvalue (`self.MaxStackSize`))
        (set `local.LocalAmount` (- _returnvalue (`self.MaxStackSize`)))
        (`KismetArrayLibrary.Array_Set` (`self.Slots`) (`local.FoundIndex`) (make `/Game/Interactables/FInventorySlot` (`local.LocalClass`) (`self.MaxStackSize`)))
        (`self.UpdateSlotAtIndex` (`local.FoundIndex`))
        (bind (_success__2 _rest) (`self.AddItem` (`local.LocalClass`) (`local.LocalAmount`)))
        (`self.UpdateCraftingMenu`)
        (return true _rest)
        (else
          (`KismetArrayLibrary.Array_Set` (`self.Slots`) (`local.FoundIndex`) (make `/Game/Interactables/FInventorySlot` (`local.LocalClass`) _returnvalue))
          (`self.UpdateSlotAtIndex` (`local.FoundIndex`))
          (return true 0)))
      (else
        (bind (_success _index_2) (`self.SearchEmptySlot`))
        (if _success
          (bind _output_get (set `local.FoundIndex` _index_2))
          (if (> (`local.LocalAmount`) (`self.MaxStackSize`))
            (`KismetArrayLibrary.Array_Set` (`self.Slots`) _output_get (make `/Game/Interactables/FInventorySlot` (`local.LocalClass`) (`self.MaxStackSize`)))
            (`self.UpdateSlotAtIndex` (`local.FoundIndex`))
            (bind (_success__3 _rest_2) (`self.AddItem` (`local.LocalClass`) (- (`local.LocalAmount`) (`self.MaxStackSize`))))
            (`self.UpdateCraftingMenu`)
            (return true _rest_2)
            (else
              (`KismetArrayLibrary.Array_Set` (`self.Slots`) (`local.FoundIndex`) (make `/Game/Interactables/FInventorySlot` (`local.LocalClass`) (`local.LocalAmount`)))
              (`self.UpdateSlotAtIndex` (`local.FoundIndex`))
              (return true 0)))
          (else
            (return false (`local.LocalAmount`))))))
    (else
      (bind (_success_2 _index_3) (`self.SearchEmptySlot`))
      (if _success_2
        (bind _output_get_2 (set `local.FoundIndex` _index_3))
        (`KismetArrayLibrary.Array_Set` (`self.Slots`) _output_get_2 (make `/Game/Interactables/FInventorySlot` (`local.LocalClass`) 1))
        (`self.UpdateSlotAtIndex` (`local.FoundIndex`))
        (if (> (`local.LocalAmount`) 1)
          (bind (_success__4 _rest_3) (`self.AddItem` (`local.LocalClass`) (- (`local.LocalAmount`) 1)))
          (`self.UpdateCraftingMenu`)
          (return true _rest_3)
          (else
            (return true 0)))
        (else
          (return false (`local.LocalAmount`)))))))

(fn `GetAmountAtIndex`
  (params (Index :type Integer))
  (returns (Amount :type Integer))
  (return (`.Amount_3_977591134B76789C8B001BB927F69178` (break `/Game/Interactables/FInventorySlot` (`KismetArrayLibrary.Array_Get` (`self.Slots`) Index)))))

(fn `GetItemInfoAtIndex`
  (params (Index :type Integer))
  (returns (`EmptySlot?` :type Boolean) (ItemInfo :type "/Game/Interactables/FItemInfo Structure") (Amount :type Integer))
  (bind (_itemclass _amount) (break `/Game/Interactables/FInventorySlot` (`KismetArrayLibrary.Array_Get` (`self.Slots`) Index)))
  (if (`KismetSystemLibrary.IsValidClass` _itemclass)
    (return false (defaults `/Game/Interactables/BP_Inventory` _itemclass) _amount)
    (else
      (return true (struct) 0))))

(fn `GetTotalAmountOfItem`
  (params (Item :type "/Game/Interactables/ItemClasses/BP_BaseItem Class Reference"))
  (returns (TotalAmount :type Integer) (SlotIndices :type "Array of Integer"))
  (locals (LocalAmount :type Integer) (LocalSlotsIndices :type "Array of Integer") (LocalItem :type "/Game/Interactables/ItemClasses/BP_BaseItem Class Reference"))
  (set `local.LocalItem` Item)
  (for (_array_element _array_index) (`self.Slots`)
    (bind (_itemclass _amount) (break `/Game/Interactables/FInventorySlot` _array_element))
    (if (`KismetSystemLibrary.IsValidClass` _itemclass)
      (if (== _itemclass (`local.LocalItem`))
        (`KismetArrayLibrary.Array_Add` (`local.LocalSlotsIndices`) _array_index)
        (set `local.LocalAmount` (+ (`local.LocalAmount`) _amount)))))
  (return (`local.LocalAmount`) (`local.LocalSlotsIndices`)))

(fn `HideInventory`
  (bind _shopwidget (`/Game/Characters/Merchant.ShopWidget` (`/Game/Characters/MainCharacterBP.NearbyMerchant` (`self.CharacterRef`))))
  (`Widget.SetVisibility` (`self.MainWidget`) "Hidden")
  (set `self.IsVisible?` false)
  (`Widget.SetIsEnabled` (`self.InventoryWidget`) false)
  (`Widget.SetVisibility` (`/Game/UI/Inventory/UI_MainWidget.ThrowWidget` (`self.MainWidget`)) "Hidden")
  (`Widget.SetIsEnabled` (`/Game/UI/Inventory/UI_Inventory.SlotPanel` (`self.InventoryWidget`)) true)
  (if (`/Game/Characters/MainCharacterBP.IsShopOpen?` (`self.CharacterRef`))
    (`Widget.SetIsEnabled` (`/Game/UI/Shop/UI_ShopWidget.GridPanel` _shopwidget) true)
    (`Widget.SetVisibility` (`/Game/UI/Shop/UI_ShopWidget.UI_SellWidget` _shopwidget) "Hidden")
    (return)
    (else
      (return))))

(fn `IsSlotEmpty?`
  (params (Index :type Integer))
  (returns (`Empty?` :type Boolean))
  (return (not (`KismetSystemLibrary.IsValidClass` (`.ItemClass_5_03A3B7174DCF4A35BEA29BBBACE0807D` (break `/Game/Interactables/FInventorySlot` (`KismetArrayLibrary.Array_Get` (`self.Slots`) Index)))))))

(fn `RemoveItem`
  (params (Item :type "/Game/Interactables/ItemClasses/BP_BaseItem Class Reference") (Amount :type Integer))
  (returns (`Success?` :type Boolean))
  (locals (LocalSlotIndicies :type "Array of Integer") (AmountToRemove :type Integer))
  (bind (_totalamount _slotindices) (`self.GetTotalAmountOfItem` Item))
  (if (>= _totalamount Amount)
    (set `local.LocalSlotIndicies` _slotindices)
    (set `local.AmountToRemove` Amount)
    (for _array_element (`local.LocalSlotIndicies`)
      (bind _amount (`self.GetAmountAtIndex` _array_element))
      (if (< _amount (`local.AmountToRemove`))
        (set `local.AmountToRemove` (- (`local.AmountToRemove`) _amount))
        (`self.RemoveItemAtIndex` _array_element _amount)
        (else
          (`self.RemoveItemAtIndex` _array_element (`local.AmountToRemove`))
          (set `local.AmountToRemove` 0)
          (break))))
    (return true)
    (else
      (return false))))

(fn `RemoveItemAtIndex`
  (params (Index :type Integer) (Amount :type Integer))
  (returns (`Success?` :type Boolean))
  (locals (LocalIndex :type Integer) (LocalAmount :type Integer))
  (bind _slots (`self.Slots`))
  (bind _localindex (`local.LocalIndex`))
  (bind (_itemclass _amount) (break `/Game/Interactables/FInventorySlot` (`KismetArrayLibrary.Array_Get` _slots _localindex)))
  (set `local.LocalIndex` Index)
  (set `local.LocalAmount` Amount)
  (if (and (not (`self.IsSlotEmpty?` (`local.LocalIndex`))) (> (`local.LocalAmount`) 0))
    (if (>= (`local.LocalAmount`) (`self.GetAmountAtIndex` (`local.LocalIndex`)))
      (`KismetArrayLibrary.Array_Set` (`self.Slots`) (`local.LocalIndex`) (make `/Game/Interactables/FInventorySlot` null))
      (`self.UpdateSlotAtIndex` (`local.LocalIndex`))
      (`self.UpdateCraftingMenu`)
      (return true)
      (else
        (`KismetArrayLibrary.Array_Set` _slots _localindex (make `/Game/Interactables/FInventorySlot` _itemclass (- _amount (`local.LocalAmount`))))
        (`self.UpdateSlotAtIndex` (`local.LocalIndex`))
        (`self.UpdateCraftingMenu`)
        (return true)))
    (else
      (return false))))

(fn `SearchEmptySlot`
  (returns (Success :type Boolean) (Index :type Integer))
  (locals (LocalBool :type Boolean) (LocalIndex :type Integer))
  (for (_array_element _array_index) (`self.Slots`)
    (if (not (`KismetSystemLibrary.IsValidClass` (`.ItemClass_5_03A3B7174DCF4A35BEA29BBBACE0807D` (break `/Game/Interactables/FInventorySlot` _array_element))))
      (set `local.LocalBool` true)
      (set `local.LocalIndex` _array_index)
      (break)))
  (return (`local.LocalBool`) (`local.LocalIndex`)))

(fn `SearchFreeStack`
  (params (ItemClass :type "/Game/Interactables/ItemClasses/BP_BaseItem Class Reference"))
  (returns (`Success?` :type Boolean) (Index :type Integer))
  (locals (LocalBool :type Boolean) (LocalIndex :type Integer))
  (for (_array_element _array_index) (`self.Slots`)
    (bind (_itemclass _amount) (break `/Game/Interactables/FInventorySlot` _array_element))
    (if (`KismetSystemLibrary.IsValidClass` _itemclass)
      (if (and (== _itemclass ItemClass) (< _amount (`self.MaxStackSize`)))
        (set `local.LocalBool` true)
        (set `local.LocalIndex` _array_index)
        (break))))
  (return (`local.LocalBool`) (`local.LocalIndex`)))

(fn `ShowInventory`
  (`Widget.SetVisibility` (`self.MainWidget`) "Visible")
  (set `PlayerController.bShowMouseCursor` true (`GameplayStatics.GetPlayerController` 0))
  (set `self.IsVisible?` true)
  (`Widget.SetIsEnabled` (`self.InventoryWidget`) true)
  (return))

(fn `UpdateCraftingMenu`
  (bind _craftingwidget (`/Game/UI/Inventory/UI_MainWidget.CraftingWidget` (`self.MainWidget`)))
  (bind _currentitemclass (`/Game/UI/Crafting/UI_CraftingMenu.CurrentItemClass` _craftingwidget))
  (if (`KismetSystemLibrary.IsValidClass` _currentitemclass)
    (`/Game/UI/Crafting/UI_CraftingMenu.UpdateDetailWindow` _craftingwidget _currentitemclass)
    (return)
    (else
      (return))))

(fn `UserConstructionScript`)